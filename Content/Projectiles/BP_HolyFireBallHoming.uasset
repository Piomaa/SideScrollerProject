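; BP_HolyFireBallHoming is a holy fireball projectile that turns toward the nearest enemy shortly after spawning.
; On BeginPlay it ignores its owner, then gathers all demon and plagued enemies.
; The nearest-target search runs inside the plagued-enemy loop, so homing requires at least one plagued enemy.
; A short non-looping timer then redirects velocity toward the target once at Speed, without continuous tracking.
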(event Custom|FindTarget
  (bind _homing_target (Variables|Default|GetHoming%20Target))
  (Utilities|Array|Clear (Variables|Default|GetHoming%20Target))
  (Utilities|FlowControl|Sequence
    (:then_0
      (bind _outactors (Actor|GetAllActorsOfClass "/Game/DamageSystem/Enemy/DemonEnemy/BP_DemonEnemy.BP_DemonEnemy_C"))
      (for _array_element _outactors
        (Utilities|Array|Add (Variables|Default|GetHoming%20Target) _array_element)))
    (:then_1
      (bind _outactors_2 (Actor|GetAllActorsOfClass "/Game/DamageSystem/Enemy/PlaguedEnemy/BP_PlaguedEnemy.BP_PlaguedEnemy_C"))
      (for _array_element_2 _outactors_2
        (Utilities|Array|Add _homing_target _array_element_2)
        (bind _output_get (Variables|Default|SetTarget (.ReturnValue (Actor|FindNearestActor (Transformation|GetActorLocation) _homing_target))))
        (Utilities|IsValid _output_get
          (:Is%20Valid
            (Utilities|Time|SetTimerbyEvent (delegate Custom|HomeTarget) 0.2)))))))

(event Custom|HomeTarget
  (bind _target (Variables|Default|GetTarget))
  (Utilities|IsValid _target
    (:Is%20Valid
      (Variables|/Script/Engine.MovementComponent|SetVelocity (Variables|Default|GetProjectileMovement) (* (Math|Vector|GetUnitDirection(Vector) (Transformation|GetActorLocation) (Transformation|GetActorLocation _target)) (Variables|Default|GetSpeed))))))

(event EventBeginPlay
  (Collision|IgnoreActorwhenMoving (Variables|Default|GetBox) (Components|GetOwner) true)
  (CallFunction|FindTarget))

(fn ConstructionScript
  (|CallParentFunction))