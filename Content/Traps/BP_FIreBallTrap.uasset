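; Fireball trap actor that launches a BP_HolyFireBall from its ProjectileLocation whenever any actor begins overlapping it, with a whoosh sound.
; It binds the fireball's hit event, damaging a struck BP_ThirdPersonCharacter and playing an explosion sound.
; The trap's mesh ignores the spawned fireball when moving.
; A separate SpawnFireBall function repeats the spawn without binding and is not called within this Blueprint.
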(event Custom|HitPlayer
  (params (SelfActor :type Actor%20Object%20Reference) (OtherActor :type Actor%20Object%20Reference) (NormalImpulse :type Vector) (Hit :type Hit%20Result%20Structure%20%28by%20ref%29))
  ;[1 1 1] Spawns fireball when actor overlaps box.If it hits player he takes damage and hit sound is played
  (bind _asbp_third_person_character (Utilities|Casting|CastToBP_ThirdPersonCharacter OtherActor))
  (Default|TakeDamage _asbp_third_person_character 1e+01)
  (Audio|PlaySound2D "/Game/Sound/Explosion_Medium_2-1.Explosion_Medium_2-1" 1.0 1.0 0.0 0 0))

(event Collision|EventActorBeginOverlap
  (params (OtherActor :type Actor%20Object%20Reference))
  ;[1 1 1] Spawns fireball when actor overlaps box.If it hits player he takes damage and hit sound is played
  (Audio|PlaySoundatLocation "/Game/Sound/Fire_Whoosh_2-15.Fire_Whoosh_2-15" (Transformation|GetActorLocation) "0, 0, 0" 1.0 1.0 0.0 0 0 0 0)
  (bind _returnvalue (Game|SpawnActorfromClass "/Game/Projectiles/BP_HolyFireBall.BP_HolyFireBall_C" (Transformation|GetWorldTransform (Variables|Default|GetProjectile%20Location)) "Undefined" "MultiplyWithRoot" self 5e+02 0.0 false 0))
  (Collision|BindEventtoOnActorHit _returnvalue (delegate Custom|HitPlayer))
  (Collision|IgnoreActorwhenMoving (Variables|Default|GetStaticMesh) _returnvalue true))

(fn ConstructionScript)

(fn SpawnFireBall
  (Game|SpawnActorfromClass "/Game/Projectiles/BP_HolyFireBall.BP_HolyFireBall_C" (Transformation|GetWorldTransform (Variables|Default|GetProjectile%20Location)) "Undefined" "MultiplyWithRoot" self 5e+02 0.0 false 0))