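; Actor component that tracks health and death state, intended for both player and enemies.
; TakeDamage subtracts the incoming damage, then either sets IsDead and fires OnDeath at zero or below, or fires OnDamageResponse.
; Heal adds health clamped between zero and MaxHealth and returns the new value.
; Both functions change nothing once IsDead is set, and the event graph holds no active logic.
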(event EventBeginPlay)

(event EventTick
  (params (DeltaSeconds :type Float%20%28single-precision%29)))

(fn Heal
  (params (Amount :type Float%20%28double-precision%29))
  ;[1 1 1] Heal Implementation
  (if (not (Variables|Default|GetisDead))
    (bind _output_get (Variables|Default|SetHealth (Math|Float|Clamp(Float) (+ Amount (Variables|Default|GetHealth)) 0.0 (Variables|Default|GetMaxHealth))))
    (return _output_get)))

(fn TakeDamage
  (params (DamageInfo :type Float%20%28double-precision%29))
  ;[1 1 1] Take Damage + Calls Events Death/OnDamage Player & Enemies inherit this
  (if (not (Variables|Default|GetisDead))
    (bind _output_get (Variables|Default|SetHealth (- (Variables|Default|GetHealth) DamageInfo)))
    (if (<= _output_get 0.0)
      (Variables|Default|SetisDead true)
      (Default|CallOnDeath)
      (else
        (Default|CallOnDamageResponse)))
    (return true)))