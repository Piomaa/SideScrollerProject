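; BP_DemonEnemy is a ranged enemy character that throws holy fireballs at the player and awards score on death.
; Attack plays a montage and, after a short delay, spawns a fireball whose hit event applies damage.
; BPCDamageSystem handles health and drives hurt audio and ragdoll death, while wrapper functions expose health, patrol route and speed.
; Navlink jumps launch the character along a suggested projectile arc, and a widget displays its health bar.
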(event Custom|Attack
  ;[1 1 1] Enemy Ranged Attack - plays animation , Spawns Fireball , Damages Player and Plays Audio
  (if (not (Variables|/Game/DamageSystem/BPC_DamageSystem.BPC_DamageSystem_C|GetisDead (Variables|Default|GetBPC_DamageSystem)))
    (Utilities|FlowControl|Sequence
      (:then_0
        (Animation|Montage|PlayMontage (Variables|Character|GetMesh) "/Game/DamageSystem/Enemy/DemonEnemy/Ranged_Enemy_Montage.Ranged_Enemy_Montage"
          (:OnCompleted
            _)
          (:OnNotifyBegin
            _))
        (Default|CallOnRangedAttackFInished))
      (:then_1
        (Utilities|FlowControl|Delay 0.5)
        (bind _returnvalue (Game|SpawnActorfromClass "/Game/Projectiles/BP_HolyFireBall.BP_HolyFireBall_C" (Transformation|GetWorldTransform (Variables|Default|GetSpawn%20Projectile%20Location)) "Undefined" "MultiplyWithRoot" self 5e+02 0.0 false 0))
        (EventDispatchers|BindEventtoOnProjectileHit _returnvalue (delegate Custom|DamagePlayer))
        (Collision|IgnoreActorwhenMoving (Variables|Collision|GetCapsuleComponent) _returnvalue true))
      (:then_2
        (Audio|PlaySound2D "/Game/Sound/Fire_Whoosh_2-15.Fire_Whoosh_2-15" 1.0 1.0 0.0 0 0)))))

(event Custom|OnDeath
  (bind _mesh (Variables|Character|GetMesh))
  ;[1 1 1] Death - Remove Physics , increase player score and play Audio
  (Utilities|FlowControl|Sequence
    (:then_0
      (Physics|SetSimulatePhysics _mesh true)
      (Collision|SetCollisionEnabled _mesh "QueryAndPhysics")
      (Components|DestroyComponent (Variables|Default|GetWidget))
      (Components|DestroyComponent (Variables|Collision|GetCapsuleComponent))
      (Utilities|FlowControl|Delay 1.6)
      (Actor|DestroyActor))
    (:then_1
      (bind _asbp_third_person_character (Utilities|Casting|CastToBP_ThirdPersonCharacter (Game|GetPlayerCharacter 0)))
      (Math|Integer|IncrementInt (Variables|/Game/Player/Blueprints/BP_ThirdPersonCharacter.BP_ThirdPersonCharacter_C|GetPlayerScore _asbp_third_person_character)))
    (:then_2
      (Audio|PlaySound2D "/Game/Sound/male-death-sound-128357.male-death-sound-128357" 0.5 1.0 0.0 0 0))))

(event Custom|OnDamageResponse
  ;[1 1 1] Damage Response - Audio
  (Audio|PlaySound2D "/Game/Sound/male_hurt7-48124_Edited.male_hurt7-48124_Edited" 1.0 1.0 0.0 0 0))

(event Custom|DamagePlayer
  (params (Other%20Actor :type Actor%20Object%20Reference) (Hit :type Hit%20Result%20Structure))
  ;[1 1 1] Enemy Ranged Attack - plays animation , Spawns Fireball , Damages Player and Plays Audio
  (Class|BPIHealth|TakeDamage(Message) Other%20Actor 25.0)
  (Audio|PlaySound2D "/Game/Sound/Explosion_Medium_2-1.Explosion_Medium_2-1" 1.0 1.0 0.0 0 0))

(event EventBeginPlay
  ;[1 1 1] Adds HealthBar
  (Utilities|FlowControl|Sequence
    (:then_0
      (bind _returnvalue (UserInterface|CreateWidget "/Game/UI/WB_EnemyHealthBar.WB_EnemyHealthBar_C" 0 self))
      (UserInterface|SetWidget (Variables|Default|GetWidget) _returnvalue))))

(event EventJumptoADestination
  (params (Destination :type Vector :default "0, 0, 0"))
  (bind (_x _y _z) (Math|Vector|BreakVector Destination))
  ;[1 1 1] Jumps To Navlink
  (bind _outlaunchvelocity (Game|SuggestProjectileVelocityCustomArc (Transformation|GetActorLocation) (Math|Vector|MakeVector _x _y (+ _z 3e+02)) 0.0 0.5))
  (Character|LaunchCharacter _outlaunchvelocity true true))

(fn ConstructionScript
  (bind _bpc_damagesystem (Variables|Default|GetBPC_DamageSystem))
  ;[1 1 1] Syncs The events between classes , if Ondeath is run in BPCDS , OnDeath will run in Demon Enemy
  (EventDispatchers|BindEventtoOnDeath _bpc_damagesystem (EventDispatchers|CreateEvent :!event Custom|OnDeath))
  (EventDispatchers|BindEventtoOnDamageResponse _bpc_damagesystem (EventDispatchers|CreateEvent :!event Custom|OnDamageResponse)))

(fn GetCurrentHealth
  (return (Variables|/Game/DamageSystem/BPC_DamageSystem.BPC_DamageSystem_C|GetHealth (Variables|Default|GetBPC_DamageSystem))))

(fn GetMaxHealth
  (return (Variables|/Game/DamageSystem/BPC_DamageSystem.BPC_DamageSystem_C|GetMaxHealth (Variables|Default|GetBPC_DamageSystem))))

(fn GetPatrolRoute
  (return (Variables|Default|GetPatrolRoute)))

(fn Heal
  (params (HealAmount :type Float%20%28double-precision%29))
  (bind _new_health (Default|Heal (Variables|Default|GetBPC_DamageSystem) HealAmount))
  (return _new_health))

(fn IsDead
  (return (Variables|/Game/DamageSystem/BPC_DamageSystem.BPC_DamageSystem_C|GetisDead (Variables|Default|GetBPC_DamageSystem))))

(fn SetMovementSpeed
  (params (Speed :type E_MovementSpeed%20Enum :default "NewEnumerator0"))
  (bind _output_get (Variables|/Script/Engine.CharacterMovementComponent|SetMaxWalkSpeed (Variables|Character|GetCharacterMovement) (Utilities|Select :Index Speed :NewEnumerator0 0.0 :NewEnumerator1 1e+02 :NewEnumerator2 2.5e+02 :NewEnumerator3 3.5e+02)))
  (return _output_get))

(fn TakeDamage
  (params (Damage%20Amount :type Float%20%28double-precision%29))
  (bind _was_damaged (Default|TakeDamage (Variables|Default|GetBPC_DamageSystem) Damage%20Amount))
  (return _was_damaged))